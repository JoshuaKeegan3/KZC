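; BP_Minty is a zombie enemy for survival mode that chases players at a randomized speed and attacks on capsule overlap.
; Game mode events report spawn and death and retarget the blackboard when players are downed or revived.
; Explosive damage routes through the radial handler, which can randomly slow it with an injury.
; Hits and kills award points, the latter by damage type, and death ragdolls it before timed removal.
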(event OnComponentBeginOverlap(Capsule)
  (params (OverlappedComponent :type Primitive%20Component%20Object%20Reference) (OtherActor :type Actor%20Object%20Reference) (OtherComp :type Primitive%20Component%20Object%20Reference) (OtherBodyIndex :type Integer) (bFromSweep :type Boolean) (SweepResult :type Hit%20Result%20Structure%20%28by%20ref%29))
  ;[1 0.1914 0.3927] Damage dealing logic
  (if (|CanAttackAndNotDead)
    (Utilities|FlowControl|DoOnce false
      (:Completed
        (Game|Damage|ApplyDamage OtherActor (Variables|Default|GetAttackDamage) (Pawn|GetController) self)))))

(event Custom|AttackPlayer
  ;[1 0.9485 0.05729] Attack Player logic
  (if (not (Variables|Default|GetIsAttacking))
    (Variables|Default|SetIsAttacking true)
    (Animation|Montage|PlayMontage (Variables|Character|GetMesh) "/Game/KZC/Minty/Animations/Zombie_Attack_Montage.Zombie_Attack_Montage" (Math|Random|RandomFloatinRange 1.0 2.0)
      (:OnCompleted
        (Variables|Default|SetIsAttacking false)
        (CallFunction|ResetAttack)))))

(event Custom|ReceivedDamge
  (params (DamageAmount :type Float%20%28double-precision%29) (DamageInstigator :type Controller%20Object%20Reference) (DamageCausingObject :type Actor%20Object%20Reference) (DamageType :type Damage%20Type%20Class%20Reference))
  ;[0.5059 1 0.5446] Zombie recieve damage logic
  (Class|BPIPointsOwner|GivePoints(Message) DamageInstigator 10)
  (if (!= (Utilities|GetClass DamageCausingObject) "BP_Minty_C")
    (bind _output_get (Variables|Default|SetHealth (- (Variables|Default|GetHealth) DamageAmount)))
    (if (and (<= _output_get 0.0) (not (Variables|Default|GetisDead)))
      ;[1 0.3216 0.3614] Death logic
      (Variables|Default|SetisDead true)
      (|GiveDeathPoints DamageType DamageInstigator
        (:out
          (Variables|Default|SetCanAttack false)
          (CallFunction|TellGameZombieDied)
          (CallFunction|UnregisterforPlayerUpdates)
          (CallFunction|ActivateRagdoll)
          (Utilities|Time|SetTimerbyEvent (delegate Custom|Delete%20Actor) 3e+01)
          ;;[0.505 1 0.9301] Stop the behaviour tree from running when we are dead, not sure of the function's side effects, i.e. if the AI controller will still be deleted
          (Class|Pawn|DetachfromControllerPendingDestroy))))))

(event Custom|PlayerRevived
  (params (Revived%20player :type Character%20Object%20Reference))
  ;[1 1 1] Find a new target to chase
  (CallFunction|UpdateBlackboardTarget Revived%20player))

(event Custom|UnregisterForPlayerUpdates
  (bind _asbp_zombie_survival_mode (Utilities|Casting|CastToBP_ZombieSurvivalMode (Game|GetGameMode)))
  (EventDispatchers|UnbindEventfromPlayerDownedNotify _asbp_zombie_survival_mode (delegate Custom|PlayerDowned))
  (EventDispatchers|UnbindEventfromPlayerRevivedNotify _asbp_zombie_survival_mode (delegate Custom|PlayerRevived)))

(event Custom|ActivateRagdoll
  (bind _mesh (Variables|Character|GetMesh))
  ;[1 1 1] Ragdoll, because we have no death animation
  (Pawn|Components|CharacterMovement|DisableMovement (Variables|Character|GetCharacterMovement))
  (Collision|SetCollisionEnabled (Variables|Character|GetMesh) "PhysicsOnly")
  (Class|SkeletalMeshComponent|SetAllBodiesSimulatePhysics _mesh true)
  (Class|SkeletalMeshComponent|SetAllBodiesPhysicsBlendWeight _mesh 1.0 false)
  (Collision|SetCollisionEnabled (Variables|Collision|GetCapsuleComponent) "NoCollision"))

(event Custom|Delete%20Actor
  ;[1 0.3216 0.3614] Death logic
  (Actor|DestroyActor))

(event Custom|ResetAttack
  ;[1 0.1914 0.3927] Damage dealing logic
  (Utilities|FlowControl|DoOnce false) ; enters at Reset
)

(event Custom|TellGameZombieSpawned
  ;[1 1 1] Death and creation book keeping events
  (Class|BPIStateMessageHandler|ZombieCreated(Message) (Game|GetGameMode)))

(event Custom|TellGameZombieDied
  ;[1 1 1] Death and creation book keeping events
  (Class|BPIStateMessageHandler|ZombieDied(Message) (Game|GetGameMode)))

(event Custom|OnTakeRadialDamage_Event
  (params (DamagedActor :type Actor%20Object%20Reference) (Damage :type Float%20%28single-precision%29) (DamageType :type Damage%20Type%20Object%20Reference) (Origin :type Vector) (HitInfo :type Hit%20Result%20Structure) (InstigatedBy :type Controller%20Object%20Reference) (DamageCauser :type Actor%20Object%20Reference))
  ;[1 1 1] Register custom damage handling events
  (|GrenadeInjuryDecision)
  (CallFunction|ReceivedDamge Damage InstigatedBy DamageCauser (Utilities|GetClass DamageType)))

(event Custom|CustomEvent_0
  (params (DamagedActor :type Actor%20Object%20Reference) (Damage :type Float%20%28single-precision%29) (DamageType :type Damage%20Type%20Object%20Reference) (InstigatedBy :type Controller%20Object%20Reference) (DamageCauser :type Actor%20Object%20Reference))
  (bind _returnvalue (Utilities|GetClass DamageType))
  (if (!= _returnvalue "/Game/KZC/Weapons/DamageTypes/BP_DamageExplosive.BP_DamageExplosive_C")
    (CallFunction|ReceivedDamge Damage InstigatedBy DamageCauser _returnvalue)
    (Development|PrintString "Hit!" true true "(R=1.000000,G=0.000000,B=0.000000,A=1.000000)")))

(event Custom|RegisterForPlayerUpdates
  (bind _asbp_zombie_survival_mode (Utilities|Casting|CastToBP_ZombieSurvivalMode (Game|GetGameMode)))
  (EventDispatchers|BindEventtoPlayerDownedNotify _asbp_zombie_survival_mode (delegate Custom|PlayerDowned))
  (EventDispatchers|BindEventtoPlayerRevivedNotify _asbp_zombie_survival_mode (delegate Custom|PlayerRevived)))

(event Custom|PlayerDowned
  (params (DownCharacter :type Character%20Object%20Reference))
  ;[1 1 1] Decide what to do when the player dies,
  ; This should make the zombie roam to random locations when the player downs
  (CallFunction|UpdateBlackboardTarget))

(event EventBeginPlay
  ;[1 1 1] Register custom damage handling events
  (EventDispatchers|BindEventtoOnTakeAnyDamage (delegate Custom|CustomEvent_0))
  (EventDispatchers|BindEventtoOnTakeRadialDamage (delegate Custom|OnTakeRadialDamage_Event))
  ;[1 1 1] Let the game mode do its book keeping
  (CallFunction|TellGameZombieSpawned)
  ;[1 1 1] Tell the Behaviour tree to chase the player
  (CallFunction|UpdateBlackboardTarget (Game|Player|GetPlayerPawn 0))
  (bind _returnvalue (CallFunction|ChooseMintySpeed))
  (Variables|/Script/Engine.CharacterMovementComponent|SetMaxWalkSpeed (Variables|Character|GetCharacterMovement) _returnvalue)
  (CallFunction|RegisterforPlayerUpdates))

(fn ConstructionScript)

(fn UpdateBlackboardTarget
  (params (NewTarget :type Object%20Object%20Reference))
  (AI|Components|Blackboard|SetValueasObject (AI|GetBlackboard 0) (Variables|Default|GetChaseTarget) NewTarget)
  (return))

(fn ChooseMintySpeed
  (if (Math|Random|RandomBoolwithWeight 0.9)
    (return (* (Variables|Default|GetSpeedBase) (Variables|Default|GetSpeedFactor)))
    (else
      (return (* (Variables|Default|GetSpeedBase) (Math|Random|RandomIntegerinRange 1 (Variables|Default|GetSpeedFactor)))))))