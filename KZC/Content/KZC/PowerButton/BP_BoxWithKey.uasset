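; Box prop for a power-button quest step that hands the employee a key.
; A start-step event arms it, after which any damage knocks the cube with a velocity impulse.
; When the armed cube hits an employee, it adds a Key to their owned items once, plays a jingle, prints a message and destroys itself.
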(event OnComponentHit(Cube)
  (params (HitComponent :type Primitive%20Component%20Object%20Reference) (OtherActor :type Actor%20Object%20Reference) (OtherComp :type Primitive%20Component%20Object%20Reference) (NormalImpulse :type Vector :default "0, 0, 0") (Hit :type Hit%20Result%20Structure%20%28by%20ref%29))
  ;[1 1 1] Set overlap state true
  (bind _asbp_employee (Utilities|Casting|CastToBP_Employee OtherActor))
  (if (and (Variables|Default|GetActive) (not (Variables|Default|GetComplete)))
    (Variables|Default|SetComplete true)
    (Utilities|Array|Add (Variables|/Game/KZC/Employee/BP_Employee.BP_Employee_C|GetOwnedItems _asbp_employee) "Key")
    (Audio|PlaySoundatLocation "/Game/RawContent/Sounds/KeyJingle.KeyJingle" (Transformation|GetActorLocation _asbp_employee) "0, 0, 0" 1.0 1.0 0.0 0 0 0 0)
    (Development|PrintString "KEY ACQUIRED")
    (Actor|DestroyActor)))

(event Custom|StartStep
  (Variables|Default|SetActive true))

(event Game|Damage|EventAnyDamage
  (params (Damage :type Float%20%28single-precision%29) (DamageType :type Damage%20Type%20Object%20Reference) (InstigatedBy :type Controller%20Object%20Reference) (DamageCauser :type Actor%20Object%20Reference))
  (if (Variables|Default|GetActive)
    (Physics|AddImpulse (Variables|Default|GetCube) "1000.000000,10.000000,50.000000" "None" true)))

(fn ConstructionScript)