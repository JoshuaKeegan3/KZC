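; BP_PowerButton is a one-shot pushable power button that prompts overlapping actors until it has been pressed.
; Interacting notifies the game mode, locks out further presses, activates the power-on audio and plays a start-up sound.
; Timelines lerp the button between its starting transform and an inward offset computed at BeginPlay, playing a click and swapping to the lit material before it springs back out.
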(event OnComponentBeginOverlap(InteractionVolume)
  (params (OverlappedComponent :type Primitive%20Component%20Object%20Reference) (OtherActor :type Actor%20Object%20Reference) (OtherComp :type Primitive%20Component%20Object%20Reference) (OtherBodyIndex :type Integer) (bFromSweep :type Boolean) (SweepResult :type Hit%20Result%20Structure%20%28by%20ref%29))
  ;[1 1 1] Player enters/exits power button influence radius
  (if (not (Variables|Default|GetHasBeenPressed))
    (Class|BPIPromptible|Prompt(Message) OtherActor (Variables|Default|GetPromptMessage) self)))

(event OnComponentEndOverlap(InteractionVolume)
  (params (OverlappedComponent :type Primitive%20Component%20Object%20Reference) (OtherActor :type Actor%20Object%20Reference) (OtherComp :type Primitive%20Component%20Object%20Reference) (OtherBodyIndex :type Integer))
  ;[1 1 1] Player enters/exits power button influence radius
  (Class|BPIPromptible|StopPrompt(Message) OtherActor))

(event EventInteract
  (params (Interactor :type Pawn%20Object%20Reference))
  (if (not (Variables|Default|GetHasBeenPressed))
    (Class|BPIStateMessageHandler|PowerButtonPushed(Message) (Game|GetGameMode))
    (Variables|Default|SetHasBeenPressed true)
    (|ButtonPressAnimationAndSound)
    (Components|Activation|Activate (Variables|Default|GetPowerOnSound) false)
    (Audio|PlaySoundatLocation "/Game/KZC/PowerButton/Audio/PowerStartUp.PowerStartUp" (Transformation|GetActorLocation) "0, 0, 0" 1.0 1.0 0.0 0 0 0 0)))

(event EventBeginPlay
  ;[1 1 1] Calculate start and end points of the button push animation
  (bind _output_get (Variables|Default|SetOutPosition (Transformation|GetRelativeTransform (Variables|Default|GetButton))))
  (Variables|Default|SetInPosition (Math|Transform|MakeTransform (- (.location _output_get) (Math|Vector|MakeVector (Variables|Default|GetDisplacement) 0.0 0.0)) (.rotation _output_get) (.scale _output_get))))

(fn ConstructionScript)