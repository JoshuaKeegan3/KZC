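; Victory door that slides open for an actor holding a purchased "Key" and triggers the win when a BP_Employee enters its victory volume.
; The interaction bounds show a prompt to key holders, and Interact re-checks the key before a one-time opening with sound.
; A timeline pushes both panels apart by offsets scaled by GapRadius, added to their current positions each update.
; The logic that disables DoorBlock and the interaction bounds is unconnected.
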(event OnComponentBeginOverlap(InteractionBounds)
  (params (OverlappedComponent :type Primitive%20Component%20Object%20Reference) (OtherActor :type Actor%20Object%20Reference) (OtherComp :type Primitive%20Component%20Object%20Reference) (OtherBodyIndex :type Integer) (bFromSweep :type Boolean) (SweepResult :type Hit%20Result%20Structure%20%28by%20ref%29))
  (bind _owneditems (Class|BPIPurchaser|GetPurchasedItems(Message) OtherActor))
  (if (Utilities|Array|ContainsItem _owneditems "Key")
    (Class|BPIPromptible|Prompt(Message) OtherActor "Press E to open" self)))

(event OnComponentEndOverlap(InteractionBounds)
  (params (OverlappedComponent :type Primitive%20Component%20Object%20Reference) (OtherActor :type Actor%20Object%20Reference) (OtherComp :type Primitive%20Component%20Object%20Reference) (OtherBodyIndex :type Integer))
  (Class|BPIPromptible|StopPrompt(Message) OtherActor))

(event OnComponentDeactivated(DoorBlock)
  (params (Component :type Actor%20Component%20Object%20Reference)))

(event OnComponentBeginOverlap(VictoryVolume)
  (params (OverlappedComponent :type Primitive%20Component%20Object%20Reference) (OtherActor :type Actor%20Object%20Reference) (OtherComp :type Primitive%20Component%20Object%20Reference) (OtherBodyIndex :type Integer) (bFromSweep :type Boolean) (SweepResult :type Hit%20Result%20Structure%20%28by%20ref%29))
  (bind _asbp_employee (Utilities|Casting|CastToBP_Employee OtherActor))
  (Default|VictoryEvent _asbp_employee))

(event Custom|Play%20Door%20Opening%20Montage
  (bind _doorleft (Variables|Default|GetDoorLeft))
  (bind _doorright (Variables|Default|GetDoorRight))
  (bind _relativelocation (Variables|/Script/Engine.SceneComponent|GetRelativeLocation _doorright))
  (bind _relativelocation_2 (Variables|/Script/Engine.SceneComponent|GetRelativeLocation _doorleft))
  (Audio|PlaySoundatLocation "/Game/KZC/PowerButton/Audio/garage_door.garage_door" (Transformation|GetActorLocation) "0, 0, 0" 1.0 1.0 0.0 0 0 0 0)
  (bind _door_offset (Timeline|Open%20Doors Play)
    (:Update
      (Transformation|SetRelativeTransform (Variables|Default|GetDoorLeft) (Math|Transform|MakeTransform (Math|Vector|MakeVector (.x _relativelocation_2) (- (.y _relativelocation_2) (* _door_offset (Variables|Default|GetGapRadius))) (.z _relativelocation_2)) (Variables|/Script/Engine.SceneComponent|GetRelativeRotation _doorleft)) false false)
      (Transformation|SetRelativeTransform _doorright (Math|Transform|MakeTransform (Math|Vector|MakeVector (.x _relativelocation) (+ (* _door_offset (Variables|Default|GetGapRadius)) (.y _relativelocation)) (.z _relativelocation)) (Variables|/Script/Engine.SceneComponent|GetRelativeRotation _doorright)) false false))))

(event EventBeginPlay
  (|Checkdoorconfigurationisvalid))

(event EventInteract
  (params (Interactor :type Pawn%20Object%20Reference))
  (bind _owneditems (Class|BPIPurchaser|GetPurchasedItems(Message) Interactor))
  (if (Utilities|Array|ContainsItem _owneditems "Key")
    (Utilities|FlowControl|DoOnce false
      (:Completed
        (CallFunction|PlayDoorOpeningMontage)))))

(fn ConstructionScript)