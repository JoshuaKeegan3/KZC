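; Interactable power button that sparks once the power event arrives and can then be pressed once to activate the next step in a chain.
; BeginPlay registers with the GameMode for that event, and the interaction volume shows a prompt while the button is active and unpressed.
; Pressing calls NextStep, removes the sparks and runs timelines that lerp the button in and back out, swapping its material and playing sounds.
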(event OnComponentBeginOverlap(InteractionVolume)
  (params (OverlappedComponent :type Primitive%20Component%20Object%20Reference) (OtherActor :type Actor%20Object%20Reference) (OtherComp :type Primitive%20Component%20Object%20Reference) (OtherBodyIndex :type Integer) (bFromSweep :type Boolean) (SweepResult :type Hit%20Result%20Structure%20%28by%20ref%29))
  ;[1 1 1] Player enters/exits power button influence radius
  (if (Variables|Default|GetActiveStep)
    (if (not (Variables|Default|GetHasBeenPressed))
      (Class|BPIPromptible|Prompt(Message) OtherActor (Variables|Default|GetPromptMessage) self))))

(event OnComponentEndOverlap(InteractionVolume)
  (params (OverlappedComponent :type Primitive%20Component%20Object%20Reference) (OtherActor :type Actor%20Object%20Reference) (OtherComp :type Primitive%20Component%20Object%20Reference) (OtherBodyIndex :type Integer))
  ;[1 1 1] Player enters/exits power button influence radius
  (Class|BPIPromptible|StopPrompt(Message) OtherActor))

(event EventPowerActivated
  (Variables|Default|SetActiveStep true)
  (CallFunction|Spark))

(event EventInteract
  (params (Interactor :type Pawn%20Object%20Reference))
  (bind _nextstep (Variables|Default|GetNextStep))
  (if (Variables|Default|GetActiveStep)
    (if (not (Variables|Default|GetHasBeenPressed))
      (Utilities|IsValid _nextstep
        (:Is%20Valid
          (Default|Activation _nextstep)
          (Components|DestroyComponent (Variables|Default|GetEmmitter))
          (Variables|Default|SetHasBeenPressed true)
          (|ButtonPressAnimationAndSound)
          ;[1 0.005208 0.005208] Play power on sound TODO
          (Components|Activation|Activate (Variables|Default|GetPowerOnSound) false))))))

(event EventBeginPlay
  ;[1 1 1] Calculate start and end points of the button push animation
  (bind _output_get (Variables|Default|SetOutPosition (Transformation|GetRelativeTransform (Variables|Default|GetButton))))
  (Variables|Default|SetInPosition (Math|Transform|MakeTransform (- (.location _output_get) (Math|Vector|MakeVector (Variables|Default|GetDisplacement) 0.0 0.0)) (.rotation _output_get) (.scale _output_get)))
  (Class|BPIPowerRegister|RegisterforPowerEvent(Message) (Game|GetGameMode) self))

(fn ConstructionScript)

(fn Spark
  (bind _returnvalue (Effects|SpawnEmitteratLocation "/Game/StarterContent/Particles/P_Sparks.P_Sparks" (Transformation|GetWorldLocation (Variables|Default|GetDefaultSceneRoot))))
  (Variables|Default|SetEmmitter _returnvalue))