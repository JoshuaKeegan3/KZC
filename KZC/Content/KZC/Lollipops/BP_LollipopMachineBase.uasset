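; Base Blueprint for lollipop machines that sell a player trait upgrade for points once the power is on.
; It registers with the game mode for the power event, which lights the machine, and its interaction volume prompts nearby actors while unpowered.
; Interaction checks power, points and prior ownership by machine name, reporting any failure to the buyer.
; A successful purchase deducts points through the game mode, then calls AwardPlayerTraitUpgrade, left empty here.
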(event OnComponentBeginOverlap(InteractionVolume)
  (params (OverlappedComponent :type Primitive%20Component%20Object%20Reference) (OtherActor :type Actor%20Object%20Reference) (OtherComp :type Primitive%20Component%20Object%20Reference) (OtherBodyIndex :type Integer) (bFromSweep :type Boolean) (SweepResult :type Hit%20Result%20Structure%20%28by%20ref%29))
  (CallFunction|ActorNearby OtherActor))

(event OnComponentEndOverlap(InteractionVolume)
  (params (OverlappedComponent :type Primitive%20Component%20Object%20Reference) (OtherActor :type Actor%20Object%20Reference) (OtherComp :type Primitive%20Component%20Object%20Reference) (OtherBodyIndex :type Integer))
  (CallFunction|PawnMovedAway OtherActor))

(event EventInteract
  (params (Interactor :type Pawn%20Object%20Reference))
  ;[0.4658 1 0.44] Called when someone tries to interact with the lollipop machine
  (CallFunction|PlayerInteracted Interactor))

(event EventPowerActivated
  ;[1 1 1] Called when the player turns on the power
  (Variables|Default|SetIsPoweredOn true)
  (CallFunction|MachinePoweredon))

(event EventBeginPlay
  ;[1 0.8923 0.4452] Register with the game mode to be notified when the power turns on
  (Class|BPIPowerRegister|RegisterforPowerEvent(Message) (Game|GetGameMode) self)
  (Rendering|SetVisibility (Variables|Default|GetPowerLight) false false))

(fn ConstructionScript)

(fn ActorNearby
  (params (NearbyActor :type Actor%20Object%20Reference))
  (if (not (Variables|Default|GetIsPoweredOn))
    (Class|BPIPromptible|Prompt(Message) NearbyActor (Utilities|String|MakeLiteralString "You must turn on the power!") self)))

(fn PawnMovedAway
  (params (NearbyActor :type Actor%20Object%20Reference))
  (Class|BPIPromptible|StopPrompt(Message) NearbyActor))

(fn MachinePoweredon
  (Rendering|SetVisibility (Variables|Default|GetPowerLight) true false))

(fn AwardPlayerTraitUpgrade
  (params (Receiver :type Actor%20Object%20Reference)))

(fn PlayerInteracted
  (params (Interactor :type Pawn%20Object%20Reference))
  (LocalVariables|SetThe%20Interactor Interactor)
  (if (Variables|Default|GetIsPoweredOn)
    ;[1 1 1] Check player has enough points
    (bind _points (Class|BPIPurchaser|GetPoints(Message) (LocalVariables|GetThe%20Interactor)))
    (if (>= _points (Variables|Default|GetPurchaseCost))
      ;[1 1 1] Check if player already has this item
      (bind _owneditems (Class|BPIPurchaser|GetPurchasedItems(Message) (LocalVariables|GetThe%20Interactor)))
      (if (not (Utilities|Array|ContainsItem _owneditems (Variables|Default|GetMachineName)))
        ;[1 1 1] This call actually deducts the points
        (Class|BPIStateMessageHandler|PlayerSpentPoints(Message) (Game|GetGameMode) (Pawn|GetController (LocalVariables|GetThe%20Interactor)) (Variables|Default|GetPurchaseCost))
        (CallFunction|AwardPlayerTraitUpgrade (LocalVariables|GetThe%20Interactor))
        (return)
        (else
          (Class|BPIPurchaser|PurchaseFailed(Message) (LocalVariables|GetThe%20Interactor) (Variables|Default|GetMachineName) "NewEnumerator2")
          (return)))
      (else
        (Class|BPIPurchaser|PurchaseFailed(Message) (LocalVariables|GetThe%20Interactor) (Variables|Default|GetMachineName) "NewEnumerator0")
        (return)))
    (else
      (Class|BPIPurchaser|PurchaseFailed(Message) (LocalVariables|GetThe%20Interactor) (Variables|Default|GetMachineName) "NewEnumerator1")
      (return))))