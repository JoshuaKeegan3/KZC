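; Orange Lollipop machine, a child Blueprint that sells the player a repeatable trait upgrade for points.
; When powered, it prompts nearby actors with the current cost.
; Each award messages the receiver to modify one trait, increments the purchase count and recalculates the cost.
; The first three prices are preset, then later ones grow exponentially from the initial cost, with an exponent offset by a constant.
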(event EventBeginPlay
  (|CallParentFunction)
  (bind _purchasecost (CallFunction|CalculatePurchaseCost (Variables|Default|GetNumbPurchases)))
  (Variables|Default|SetPurchaseCost _purchasecost))

(fn ConstructionScript)

(fn ActorNearby
  (params (NearbyActor :type Actor%20Object%20Reference))
  (|CallParentFunction NearbyActor)
  (if (Variables|Default|GetIsPoweredOn)
    (Class|BPIPromptible|Prompt(Message) NearbyActor (Utilities|String|Append (Utilities|String|Append (Variables|Default|GetPromptMessage) (Utilities|String|ToString(Integer) (Variables|Default|GetPurchaseCost))) " Points") self)))

(fn CalculatePurchaseCost
  (params (NumbPurchases :type Integer))
  (switch int NumbPurchases
    (:Default
      (return (Math|Float|Truncate (* (Variables|Default|Getinitial%20cost) (Math|Float|Power (+ (Class|KismetSystemLibrary|MakeLiteralInteger 1) (Variables|Default|Getgrowth%20rate)) (Math|Conversions|ToFloat(Integer) (+ NumbPurchases (Class|KismetSystemLibrary|MakeLiteralInteger 7))))))))
    (:0
      (return (Variables|Default|Getinitial%20cost)))
    (:1
      (return (Variables|Default|Getsecond%20cost)))
    (:2
      (return (Variables|Default|Getthird%20cost)))))

(fn AwardPlayerTraitUpgrade
  (params (Receiver :type Actor%20Object%20Reference))
  (|CallParentFunction Receiver)
  (Class|BPIPlayerTraits|PlayerTraitModified(Message) Receiver "NewEnumerator4" 1 0.0 false (Variables|Default|GetMachineName))
  (bind _result (Math|Integer|IncrementInt (Variables|Default|GetNumbPurchases))
    (:%20%20
      (bind _purchasecost (CallFunction|CalculatePurchaseCost _result))
      (Variables|Default|SetPurchaseCost _purchasecost))))