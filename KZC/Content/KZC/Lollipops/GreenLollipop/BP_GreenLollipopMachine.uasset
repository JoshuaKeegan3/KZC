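; BP_GreenLollipopMachine is a purchasable lollipop vending machine that upgrades a player's reload trait.
; It extends a parent machine class, calling the parent logic in each override.
; When a player is nearby and the machine is powered, it sends them a prompt showing the point cost.
; On award, it messages the receiver with the reload multiplier and the machine name as vendor.
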(event EventBeginPlay
  (|CallParentFunction))

(fn ConstructionScript)

(fn ActorNearby
  (params (NearbyActor :type Actor%20Object%20Reference))
  (|CallParentFunction NearbyActor)
  (if (Variables|Default|GetIsPoweredOn)
    (Class|BPIPromptible|Prompt(Message) NearbyActor (Utilities|String|Append (Utilities|String|Append (Variables|Default|GetPromptMessage) (Utilities|String|ToString(Integer) (Variables|Default|GetPurchaseCost))) " Points") self)))

(fn AwardPlayerTraitUpgrade
  (params (Receiver :type Actor%20Object%20Reference))
  (|CallParentFunction Receiver)
  (Class|BPIPlayerTraits|PlayerTraitModified(Message) Receiver "NewEnumerator1" 0 (Variables|Default|GetReloadMultiplier) true (Variables|Default|GetMachineName)))