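; Red Lollipop vending machine, a child of a machine base Blueprint, that sells a player health upgrade for points.
; BeginPlay sets its name and purchase cost before calling the parent, and when powered it prompts nearby actors with that cost.
; Awarding the upgrade sends the new health value and machine name to the receiver, then runs the parent logic.
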(event EventBeginPlay
  ;[1 1 1] Set this machine's name
  (Variables|Default|SetMachineName "RedLollipop")
  (Variables|Default|SetPurchaseCost 2500)
  (|CallParentFunction))

(fn ConstructionScript)

(fn ActorNearby
  (params (NearbyActor :type Actor%20Object%20Reference))
  (|CallParentFunction NearbyActor)
  (if (Variables|Default|GetIsPoweredOn)
    (Class|BPIPromptible|Prompt(Message) NearbyActor (Utilities|String|Append (Utilities|String|Append (Variables|Default|GetPromptMessage) (Utilities|String|ToString(Integer) (Variables|Default|GetPurchaseCost))) " Points") self)))

(fn MachinePoweredon
  (|CallParentFunction))

(fn AwardPlayerTraitUpgrade
  (params (Receiver :type Actor%20Object%20Reference))
  (Class|BPIPlayerTraits|PlayerTraitModified(Message) Receiver "NewEnumerator0" (Variables|Default|GetNewHealthValue) 0.0 false (Variables|Default|GetMachineName))
  (|CallParentFunction Receiver))