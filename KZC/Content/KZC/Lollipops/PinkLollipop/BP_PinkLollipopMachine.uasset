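; BP_PinkLollipopMachine is a lollipop vending machine that sells a damage upgrade to players for points.
; It extends a parent machine class, deferring to it on begin play, proximity and award.
; When powered, it shows a nearby actor a prompt with the purchase cost.
; On award, it messages the receiver with the trait, damage multiplier and vendor name before running the parent's award logic.
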(event EventBeginPlay
  (|CallParentFunction))

(fn ConstructionScript)

(fn ActorNearby
  (params (NearbyActor :type Actor%20Object%20Reference))
  (|CallParentFunction NearbyActor)
  (if (Variables|Default|GetIsPoweredOn)
    (Class|BPIPromptible|Prompt(Message) NearbyActor (Utilities|String|Append (Utilities|String|Append (Utilities|String|MakeLiteralString "Deal More Damage: ") (Utilities|String|ToString(Integer) (Variables|Default|GetPurchaseCost))) " Points") self)))

(fn AwardPlayerTraitUpgrade
  (params (Receiver :type Actor%20Object%20Reference))
  (Class|BPIPlayerTraits|PlayerTraitModified(Message) Receiver "NewEnumerator3" 0 (Variables|Default|GetDamageMultiplier) true (Variables|Default|GetMachineName))
  (|CallParentFunction Receiver))