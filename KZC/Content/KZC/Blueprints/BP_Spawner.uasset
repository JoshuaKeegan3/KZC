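; BP_Spawner is a placed spawn point that creates zombies at its own transform.
; SpawnZombie forwards health and speed factor to MakeZombie, which always spawns the hard-coded BP_Minty class, using ZombieToSpawn only as a validity check.
; Debug prints report spawns or a missing class by spawner name.
; Helper functions expose the spawner's name and its distance to the first player's pawn.
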(event Custom|MakeZombie
  (params (Health :type Float%20%28double-precision%29) (SpeedFactor :type Integer))
  (if (Utilities|IsValidClass (Variables|Default|GetZombieToSpawn))
    (Game|SpawnActorfromClass "/Game/KZC/Minty/BP_Minty.BP_Minty_C" (Transformation|GetActorTransform) "AlwaysSpawn" 0 Health SpeedFactor 0)
    (Development|PrintString (Utilities|String|Append (Utilities|String|ToString(Name) (Variables|Default|GetSpawnerName)) (Utilities|String|MakeLiteralString ": ran spawn code!")))
    (else
      ;[1 1 1] Debug message
      (Development|PrintString (Utilities|String|Append (Utilities|String|Append (Utilities|String|MakeLiteralString "Spawner: ") (Utilities|String|ToString(Name) (Variables|Default|GetSpawnerName))) " Has no class to spawn ")))))

(event EventSpawnZombie
  (params (Health :type Float%20%28double-precision%29) (SpeedFactor :type Integer))
  (CallFunction|MakeZombie Health SpeedFactor))

(fn ConstructionScript)

(fn GetDistancetoPlayer
  (return (Math|Vector|Distance(Vector) (Transformation|GetActorLocation) (Transformation|GetActorLocation (Game|Player|GetPlayerPawn 0)))))

(fn GetSpawnerName
  (return (Variables|Default|GetSpawnerName)))