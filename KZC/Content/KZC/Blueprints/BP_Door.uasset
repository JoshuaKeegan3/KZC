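; Purchasable zombie-mode door that players open with points to activate its two linked zones, ZoneA and ZoneB.
; Overlapping InteractionBounds shows a price prompt; Interact checks the player's BP_ZombiePlayerState points, sending a failure message if short.
; Opening reports the spend and zone activations to the GameMode, disables the blocker and trigger, then swings the mesh via a timeline.
; BeginPlay prints a warning if either zone is unset.
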(event OnComponentBeginOverlap(InteractionBounds)
  (params (OverlappedComponent :type Primitive%20Component%20Object%20Reference) (OtherActor :type Actor%20Object%20Reference) (OtherComp :type Primitive%20Component%20Object%20Reference) (OtherBodyIndex :type Integer) (bFromSweep :type Boolean) (SweepResult :type Hit%20Result%20Structure%20%28by%20ref%29))
  (if (not (Variables|Default|GetisOpen))
    (Class|BPIPromptible|Prompt(Message) OtherActor (|Makepromptmessage) self)))

(event OnComponentEndOverlap(InteractionBounds)
  (params (OverlappedComponent :type Primitive%20Component%20Object%20Reference) (OtherActor :type Actor%20Object%20Reference) (OtherComp :type Primitive%20Component%20Object%20Reference) (OtherBodyIndex :type Integer))
  (Class|BPIPromptible|StopPrompt(Message) OtherActor))

(event OnComponentDeactivated(DoorBlock)
  (params (Component :type Actor%20Component%20Object%20Reference)))

(event Custom|OpenDoor
  (params (Opener :type Controller%20Object%20Reference))
  (bind _returnvalue (Game|GetGameMode))
  (bind _returnvalue_2 (Game|GetGameMode))
  (bind _doorblock (Variables|Default|GetDoorBlock))
  (|debugmessage)
  ;[1 1 1] subtract points from player
  (Utilities|IsValid _returnvalue_2
    (:Is%20Valid
      (Class|BPIStateMessageHandler|PlayerSpentPoints(Message) _returnvalue_2 Opener (Variables|Default|GetPrice)))
    (:Is%20Not%20Valid
      _))
  ;[1 1 1] activate zones
  (Variables|/Game/KZC/Blueprints/BP_Zone.BP_Zone_C|SetIsActive (Variables|Default|GetZoneA) true)
  (Variables|/Game/KZC/Blueprints/BP_Zone.BP_Zone_C|SetIsActive (Variables|Default|GetZoneB) true)
  ;[1 1 1] tell the world that the door opened
  (Utilities|IsValid _returnvalue
    (:Is%20Valid
      (Class|BPIZoneStateMessage|ZoneActivated(Message) _returnvalue (Variables|Default|GetZoneA))
      (Class|BPIZoneStateMessage|ZoneActivated(Message) _returnvalue (Variables|Default|GetZoneB))
      ;[1 1 1] Stop responding to interaction events
      (Variables|Default|SetisOpen true)
      ;[1 1 1] Stop responding to overlaps
      (Components|Activation|Deactivate (Variables|Default|GetInteractionBounds))
      (Collision|SetCollisionEnabled _doorblock "NoCollision")
      ;[1 1 1] remove barrier to player
      (Components|Activation|Deactivate _doorblock)
      ;[1 1 1] play door opening montage
      (CallFunction|PlayDoorOpeningMontage))))

(event Custom|Play%20Door%20Opening%20Montage
  (Development|PrintString "playing door opening anim" true true "(R=0.169885,G=1.000000,B=0.124194,A=1.000000)")
  (bind _rotationsequence (Timeline|OpenDoorTimeline Play)
    (:Update
      (Transformation|SetRelativeRotation (Variables|Default|GetDoorMesh) (Math|Rotator|MakeRotator 0.0 0.0 (* _rotationsequence (Variables|Default|Getfinal%20angle))) false false))))

(event EventBeginPlay
  (|Checkdoorconfigurationisvalid))

(event EventInteract
  (params (Interactor :type Pawn%20Object%20Reference))
  (bind _returnvalue (Pawn|GetController Interactor))
  (bind _playerstate (Variables|/Script/Engine.Controller|GetPlayerState _returnvalue))
  (if (not (Variables|Default|GetisOpen))
    ;[1 1 1] If there is no player state, the controller is not a human controller...
    (Utilities|IsValid _playerstate
      (:Is%20Valid
        ;[1 1 1] Currently assuming we are using the custom state class
        (bind _asbp_zombie_player_state (Utilities|Casting|CastToBP_ZombiePlayerState _playerstate))
        (if (>= (Variables|/Game/KZC/Blueprints/Framework/BP_ZombiePlayerState.BP_ZombiePlayerState_C|GetPoints _asbp_zombie_player_state) (Variables|Default|GetPrice))
          (CallFunction|OpenDoor _returnvalue)
          (Class|BPIPromptible|StopPrompt(Message) Interactor)
          (else
            (Class|BPIPurchaser|PurchaseFailed(Message) Interactor (Variables|Default|GetDoorName) "NewEnumerator0")))))))

(fn ConstructionScript)