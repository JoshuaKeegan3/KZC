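; BP_BigDoor is a two-mesh door that slides upward and disappears when its PlayDoorOpeningMontage event is called.
; The ZoomUpMagic timeline outputs a LocationOffset that is scaled by FinalAngle and added to each mesh's current relative Z on every update, so movement accumulates per tick.
; When the timeline finishes, both meshes are hidden; nothing in the graph changes collision or closes the door again.
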(event EventBeginPlay
  (|CallParentFunction) ; This node is disabled and will not be called.\nDrag off pins to build functionality.
)

(event Collision|EventActorBeginOverlap
  (params (OtherActor :type Actor%20Object%20Reference)))

(event EventTick
  (params (DeltaSeconds :type Float%20%28single-precision%29)))

(event EventPlayDoorOpeningMontage
  (bind _doormesh (Variables|Default|GetDoorMesh))
  (bind _sm_bld_containerbridge_door_02 (Variables|Default|GetSM_Bld_ContainerBridge_Door_02))
  (bind _relativelocation (Variables|/Script/Engine.SceneComponent|GetRelativeLocation _sm_bld_containerbridge_door_02))
  (bind _relativelocation_2 (Variables|/Script/Engine.SceneComponent|GetRelativeLocation _doormesh))
  (bind _locationoffset (Timeline|ZoomUpMagic Play)
    (:Update
      (Transformation|SetRelativeLocation _doormesh (Math|Vector|MakeVector (.x _relativelocation_2) (.y _relativelocation_2) (+ (.z _relativelocation_2) (* _locationoffset (Variables|Default|Getfinal%20angle)))) false false)
      (Transformation|SetRelativeLocation _sm_bld_containerbridge_door_02 (Math|Vector|MakeVector (.x _relativelocation) (.y _relativelocation) (+ (.z _relativelocation) (* _locationoffset (Variables|Default|Getfinal%20angle)))) false false))
    (:Finished
      (Rendering|SetVisibility (Variables|Default|GetDoorMesh) false false)
      (Rendering|SetVisibility (Variables|Default|GetSM_Bld_ContainerBridge_Door_02) false false))))

(fn ConstructionScript
  (|CallParentFunction))