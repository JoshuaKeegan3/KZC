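; Game mode for round-based zombie survival, running a Preround, Round and GameOver state machine on Tick with timed breaks between rounds.
; BP_ZombieWorldState holds kill counts and per-round zombie scaling; a round ends when kills match its quota.
; Spawning uses random capped batches, alternating between the first player-occupied zone and its active adjacent zones.
; It also handles point spending, power activation broadcasts and zone, death, down and revive notifications.
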(event EventPlayerSpentPoints
  (params (Spender :type Controller%20Object%20Reference) (PointsSpent :type Integer))
  (bind _asbp_zombie_player_state (Utilities|Casting|CastToBP_ZombiePlayerState (Variables|/Script/Engine.Controller|GetPlayerState Spender)))
  (Variables|/Game/KZC/Blueprints/Framework/BP_ZombiePlayerState.BP_ZombiePlayerState_C|SetPoints _asbp_zombie_player_state (- (Variables|/Game/KZC/Blueprints/Framework/BP_ZombiePlayerState.BP_ZombiePlayerState_C|GetPoints _asbp_zombie_player_state) PointsSpent))
  (bind _asbp_employee_controller (Utilities|Casting|CastToBP_EmployeeController Spender))
  (Default|PointsUpdated _asbp_employee_controller)
  (Audio|PlaySound2D "/Game/RawContent/Sounds/general_purchase.general_purchase" 1.0 1.0 0.0 0 0))

(event EventZoneActivated
  (params (TheZone :type BP%20Zone%20Object%20Reference))
  ;[1 1 1] Pass the message along to the game state that a zone was activated
  (Class|BPIZoneStateMessage|ZoneActivated(Message) (Game|GetGameState) TheZone))

(event EventPowerButtonPushed
  ;[1 0.9894 0.1875] Power System
  (for _array_element (Variables|Default|GetPoweredActors)
    (Default|PowerActivated _array_element))
  (Development|PrintString "Power Activated!" true true "(R=0.937526,G=1.000000,B=0.005208,A=1.000000)"))

(event EventRegisterforPowerEvent
  (params (ActorToNotify :type BPI%20Powered%20Actor%20Interface))
  ;[1 0.9894 0.1875] Power System
  (Utilities|Array|Add (Variables|Default|GetPoweredActors) ActorToNotify))

(event EventZombieCreated
  ;[1 1 1] Update number of zombies alive variable when this event is recieved
  (Math|Integer|IncrementInt (Variables|/Game/KZC/Blueprints/Framework/BP_ZombieWorldState.BP_ZombieWorldState_C|GetAliveZombies (Variables|Default|Getstate))))

(event EventPlayerDowned
  (params (DownedPlayer :type Character%20Object%20Reference))
  (Default|CallPlayerDownedNotify DownedPlayer))

(event EventPlayerRevived
  (params (RevivedPlayer :type Character%20Object%20Reference))
  (Default|CallPlayerRevivedNotify RevivedPlayer))

(event EventEndGame
  ;[1 1 1] Update state
  (Variables|Default|SetGame_State "NewEnumerator2"))

(event EventPlayerDied
  ;[1 1 1] Update state
  (Variables|Default|SetGame_State "NewEnumerator2"))

(event EventZombieDied
  (bind _state (Variables|Default|Getstate))
  ;[1 1 1] Mutate world state
  (Math|Integer|DecrementInt (Variables|/Game/KZC/Blueprints/Framework/BP_ZombieWorldState.BP_ZombieWorldState_C|GetAliveZombies _state)
    (:%20%20
      (Math|Integer|IncrementInt (Variables|/Game/KZC/Blueprints/Framework/BP_ZombieWorldState.BP_ZombieWorldState_C|GetZombiesKilled _state)
        (:%20%20
          (Default|CallZombieDiedNotifier)
          (bind _shouldroundend (CallFunction|CheckRoundOver))
          (if _shouldroundend
            (CallFunction|EndRound)))))))

(event EventBeginPlay
  (bind _returnvalue (Game|GetGameState))
  ;[1 1 1] Store a reference to the world state
  (Utilities|IsValid _returnvalue
    (:Is%20Valid
      (bind _asbp_zombie_world_state (Utilities|Casting|CastToBP_ZombieWorldState _returnvalue))
      (Variables|Default|Setstate _asbp_zombie_world_state)
      ;[1 1 1] World state inits round to 0 on construction
      (CallFunction|EndRound))))

(event EventTick
  (params (DeltaSeconds :type Float%20%28single-precision%29))
  ;[1 1 1] State machine activities go here
  (switch Utilities|FlowControl|Switch|SwitchonE_GameStates (Variables|Default|GetGame_State)
    (:NewEnumerator0
      (Audio|PlaySound2D "/Game/RawContent/Sounds/Clock_tick.Clock_tick" 1.0 1.0 0.0 0 0))
    (:NewEnumerator1
      (CallFunction|RunZombieSpawnLogic))))

(event Custom|EndRound
  (Variables|Default|SetGame_State "NewEnumerator0")
  (Utilities|Time|SetTimerbyEvent (delegate Custom|StartNextRound) (Variables|Default|GetInterRoundTimer))
  (Default|ResetFields (Variables|Default|Getstate))
  (Default|CallRoundEnded)
  (Audio|PlaySound2D "/Game/RawContent/Sounds/clown-laugh.clown-laugh" 1.0 1.0 0.0 0 0))

(event Custom|StartNextRound
  (bind _state (Variables|Default|Getstate))
  (bind _result (Math|Integer|IncrementInt (Variables|/Game/KZC/Blueprints/Framework/BP_ZombieWorldState.BP_ZombieWorldState_C|GetCurrentRound _state))
    (:%20%20
      (Default|CalculateZombieHealth _state)
      (Default|CalculateZombiesThisWave _state)
      (Default|CalculateMaxZombieSpeedThisWave _state)
      (Variables|Default|SetGame_State "NewEnumerator1")
      (Default|CallRoundChanged _result))))

(event Custom|RunZombieSpawnLogic
  (Development|PrintString "Trying to spawn zombies!")
  (CallFunction|SpawnZombies))

(fn ConstructionScript
  ;[1 1 1] Set initial game state when game mode is created
  (Variables|Default|SetGame_State "NewEnumerator0"))

(fn GetBatchSize
  (bind _state (Variables|Default|Getstate))
  (bind _state_2 (Variables|Default|Getstate))
  ;[1 1 1] Determine how many zombies spawned so far
  (bind _output_get (LocalVariables|SetTotalZombiesSpawned (+ (Variables|/Game/KZC/Blueprints/Framework/BP_ZombieWorldState.BP_ZombieWorldState_C|GetAliveZombies _state) (Variables|/Game/KZC/Blueprints/Framework/BP_ZombieWorldState.BP_ZombieWorldState_C|GetZombiesKilled _state))))
  ;[1 1 1] Determine how many zombies we could spawn
  (bind _output_get_2 (LocalVariables|SetZombiesLeft (Math|Integer|Min(Integer) (- (Variables|Default|GetMaxAliveZombies) (Variables|/Game/KZC/Blueprints/Framework/BP_ZombieWorldState.BP_ZombieWorldState_C|GetAliveZombies (Variables|Default|Getstate))) (- (Variables|/Game/KZC/Blueprints/Framework/BP_ZombieWorldState.BP_ZombieWorldState_C|GetZombiesThisRound _state_2) _output_get))))
  (Development|PrintString (Utilities|String|Append (Utilities|String|MakeLiteralString "Max potential spawnable zombies: ") (Utilities|String|ToString(Integer) _output_get_2)))
  (if (<= (Variables|/Game/KZC/Blueprints/Framework/BP_ZombieWorldState.BP_ZombieWorldState_C|GetCurrentRound _state_2) (Variables|/Game/KZC/Blueprints/Framework/BP_ZombieWorldState.BP_ZombieWorldState_C|GetMaxEarlyRound _state_2))
    ;[1 1 1] If it's a low round make smaller batches
    (return (Math|Random|RandomIntegerinRange 0 (Math|Integer|Min(Integer) (LocalVariables|GetZombiesLeft) 2)))
    (else
      ;[1 1 1] If it's a high round spawn 0 to 4 zombies in a batch
      (return (Math|Random|RandomIntegerinRange 0 (Math|Integer|Min(Integer) (LocalVariables|GetZombiesLeft) 4))))))

(fn SpawnZombies
  (LocalVariables|SetZoneWithPlayer (Utilities|Array|Get(acopy) (Variables|/Game/KZC/Blueprints/Framework/BP_ZombieWorldState.BP_ZombieWorldState_C|GetZonesWithPlayers (Variables|Default|Getstate))))
  (LocalVariables|SetHealthThisBatch (Variables|/Game/KZC/Blueprints/Framework/BP_ZombieWorldState.BP_ZombieWorldState_C|GetZombieHealth (Variables|Default|Getstate)))
  (bind _batchsize (CallFunction|GetBatchSize))
  (bind _output_get (LocalVariables|SetZombiesLeftToSpawn _batchsize))
  (if (> _output_get 0)
    (if (Variables|Default|GetShouldHere)
      (Variables|Default|SetShouldHere (not (Variables|Default|GetShouldHere)))
      ;[1 1 1] Check player zone has spawner
      (if (Utilities|Array|IsNotEmpty (Variables|/Game/KZC/Blueprints/BP_Zone.BP_Zone_C|GetSpawners (LocalVariables|GetZoneWithPlayer)))
        (while (> (LocalVariables|GetZombiesLeftToSpawn) 0) :!label _label
          (Default|SpawnZombie (LocalVariables|GetZoneWithPlayer) (LocalVariables|GetHealthThisBatch) (Variables|/Game/KZC/Blueprints/Framework/BP_ZombieWorldState.BP_ZombieWorldState_C|GetMaxZombieSpeedFactor (Variables|Default|Getstate)))
          (Math|Integer|DecrementInt (LocalVariables|GetZombiesLeftToSpawn)))
        (else
          ;[1 1 1] Spawn zombies in adjacent zones
          (bind _zonestospawnin (CallFunction|FindAdjacentActiveZones (LocalVariables|GetZoneWithPlayer) :!label _label_2))
          (if (Utilities|Array|IsNotEmpty _zonestospawnin)
            (bind _array_element (Utilities|Array|ForEachLoopwithBreak _zonestospawnin :!label _label_3)
              (:LoopBody
                (Default|SpawnZombie _array_element (LocalVariables|GetHealthThisBatch) (Variables|/Game/KZC/Blueprints/Framework/BP_ZombieWorldState.BP_ZombieWorldState_C|GetMaxZombieSpeedFactor (Variables|Default|Getstate)))
                (Math|Integer|DecrementInt (LocalVariables|GetZombiesLeftToSpawn)
                  (:%20%20
                    (if (not (> (LocalVariables|GetZombiesLeftToSpawn) 0))
                      (goto _label_3 Break)))))
              (:Completed
                (if (> (LocalVariables|GetZombiesLeftToSpawn) 0)
                  (goto _label_3))))
            (else
              (goto _label)))))
      (else
        (Variables|Default|SetShouldHere (not (Variables|Default|GetShouldHere)))
        (goto _label_2)))
    (else
      (return))))

(fn TrySpawnZombie
  (params (Zone :type BP%20Zone%20Object%20Reference))
  (bind _spawners (Variables|/Game/KZC/Blueprints/BP_Zone.BP_Zone_C|GetSpawners Zone))
  (bind _returnvalue (Utilities|Array|IsNotEmpty _spawners))
  (if _returnvalue
    (Default|SpawnZombie Zone 0.0))
  (return _returnvalue))

(fn FindAdjacentActiveZones
  (params (Zone :type BP%20Zone%20Object%20Reference))
  (for _array_element (Variables|/Game/KZC/Blueprints/BP_Zone.BP_Zone_C|GetAdjacentZones Zone)
    ;[1 1 1] Zone has spawners and is active
    (if (and (Variables|/Game/KZC/Blueprints/BP_Zone.BP_Zone_C|GetIsActive _array_element) (Utilities|Array|IsNotEmpty (Variables|/Game/KZC/Blueprints/BP_Zone.BP_Zone_C|GetSpawners _array_element)))
      (Utilities|Array|Add (LocalVariables|GetAnswer) _array_element)))
  (return (LocalVariables|GetAnswer)))

(fn CheckRoundOver
  (bind _state (Variables|Default|Getstate))
  (return (== (Variables|/Game/KZC/Blueprints/Framework/BP_ZombieWorldState.BP_ZombieWorldState_C|GetZombiesThisRound _state) (Variables|/Game/KZC/Blueprints/Framework/BP_ZombieWorldState.BP_ZombieWorldState_C|GetZombiesKilled _state))))