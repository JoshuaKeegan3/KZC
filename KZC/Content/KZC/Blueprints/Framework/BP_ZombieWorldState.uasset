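; World state for a round-based zombie mode, holding per-round difficulty values, zombie counters and the zones that players occupy.
; Zone enter and leave events add and remove entries in the occupied-zone list.
; Health and wave size build on their previous values, with early-round rules giving way to multiplicative health and round-scaled count growth after MaxEarlyRound.
; Maximum speed follows a stepped round lookup, and ResetFields clears alive and killed counts.
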(event EventBeginPlay)

(event EventTick
  (params (DeltaSeconds :type Float%20%28single-precision%29)))

(event EventPlayerEnteredZone
  (params (TheZone :type BP%20Zone%20Object%20Reference))
  (Utilities|Array|Add (Variables|Default|GetZonesWithPlayers) TheZone))

(event EventPlayerLeftZone
  (params (TheZone :type BP%20Zone%20Object%20Reference))
  (Utilities|Array|RemoveItem (Variables|Default|GetZonesWithPlayers) TheZone))

(event EventZoneActivated
  (params (TheZone :type BP%20Zone%20Object%20Reference))
  ;[1 1 1] This could be used if we want to keep a list of all active zones
)

(fn ConstructionScript)

(fn CalculateZombieHealth
  (if (<= (Variables|Default|GetCurrentRound) (Variables|Default|GetMaxEarlyRound))
    (Variables|Default|SetZombieHealth (+ (LocalVariables|GetHardcodeIncrement) (Variables|Default|GetZombieHealth)))
    (else
      (Variables|Default|SetZombieHealth (* (Variables|Default|GetZombieHealth) (Variables|Default|GetHealthCurve))))))

(fn CalculateZombiesThisWave
  (bind _currentround (Variables|Default|GetCurrentRound))
  (switch int _currentround
    (:Default
      (if (> _currentround (Variables|Default|GetMaxEarlyRound))
        (Variables|Default|SetZombiesThisRound (Math|Float|Round (+ (Math|Conversions|ToFloat(Integer) (Variables|Default|GetZombiesThisRound)) (* (Math|Conversions|ToFloat(Integer) (Variables|Default|GetCurrentRound)) (LocalVariables|Getround%20factor)))))))
    (:5
      ;[1 1 1] On round 11 switch to algorithm
      (Variables|Default|SetZombiesThisRound (+ (Variables|Default|GetZombiesThisRound) 1)))
    (:6
      ;;[1 1 1] on round 6 add 2 to zombies this wave
      ;;;[1 1 1] on round 5 add 1 to zombies this wave
      (Variables|Default|SetZombiesThisRound (+ (Variables|Default|GetZombiesThisRound) 2)))))

(fn CalculateMaxZombieSpeedThisWave
  (bind _speedfactor (CallFunction|GetSpeedFactor (Variables|Default|GetCurrentRound)))
  (Variables|Default|SetMaxZombieSpeedFactor _speedfactor))

(fn GetSpeedFactor
  (params (Round :type Integer))
  (switch int Round
    (:Default
      (return 6))
    (:0
      _)
    (:1
      _)
    (:2
      _)
    (:3
      (return 2))
    (:4
      (return 4))
    (:5
      (return 4))
    (:6
      (return 4))
    (:7
      (return 5)))
  (return 1))

(fn ResetFields
  (Variables|Default|SetAliveZombies 0)
  (Variables|Default|SetZombiesKilled 0))