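; BP_Zone is a named map zone that tracks player presence and spawns zombies through its associated spawners.
; ZoneBounds overlaps by player-controlled characters report zone entry and exit to the game state, and a zone flagged active also reports entry on BeginPlay.
; SpawnZombie forwards health and speed factor to a randomly chosen spawner, printing a zone-prefixed debug message when none are associated.
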(event OnComponentBeginOverlap(ZoneBounds)
  (params (OverlappedComponent :type Primitive%20Component%20Object%20Reference) (OtherActor :type Actor%20Object%20Reference) (OtherComp :type Primitive%20Component%20Object%20Reference) (OtherBodyIndex :type Integer) (bFromSweep :type Boolean) (SweepResult :type Hit%20Result%20Structure%20%28by%20ref%29))
  ;[1 1 1] @TODO notify systems when the player enters the zone
  (bind _ascharacter (Utilities|Casting|CastToCharacter OtherActor))
  (if (Pawn|IsPlayerControlled _ascharacter)
    (CallFunction|PlayerEnteredZone)
    (CallFunction|PrintInfo "character entered zone")))

(event OnComponentEndOverlap(ZoneBounds)
  (params (OverlappedComponent :type Primitive%20Component%20Object%20Reference) (OtherActor :type Actor%20Object%20Reference) (OtherComp :type Primitive%20Component%20Object%20Reference) (OtherBodyIndex :type Integer))
  ;[1 1 1] @TODO notify systems when the player enters the zone
  (bind _ascharacter (Utilities|Casting|CastToCharacter OtherActor))
  (if (Pawn|IsPlayerControlled _ascharacter)
    (CallFunction|PlayerLeftZone)
    (CallFunction|PrintInfo "character left zone")))

(event Custom|ChooseSpawner
  (params (Health :type Float%20%28double-precision%29) (SpeedFactor :type Integer))
  (bind _spawners (Variables|Default|GetSpawners))
  ;[1 1 1] Simple spawn algorithm, choose a random spawner
  (if (Utilities|Array|IsNotEmpty _spawners)
    (Default|SpawnZombie (Utilities|Array|Get(acopy) (Variables|Default|GetSpawners) (Math|Random|RandomInteger (Utilities|Array|Length _spawners))) Health SpeedFactor)
    (else
      (CallFunction|PrintInfo "No spawners associated!"))))

(event Custom|PlayerEnteredZone
  ;[1 1 1] Tell the game state when the player enters and leaves this zone
  (Class|BPIZoneStateMessage|PlayerEnteredZone(Message) (Game|GetGameState) self))

(event Custom|PlayerLeftZone
  ;[1 1 1] Tell the game state when the player enters and leaves this zone
  (Class|BPIZoneStateMessage|PlayerLeftZone(Message) (Game|GetGameState) self))

(event EventSpawnZombie
  (params (Health :type Float%20%28double-precision%29) (SpeedFactor :type Integer))
  (CallFunction|ChooseSpawner Health SpeedFactor))

(event EventBeginPlay
  (if (Variables|Default|GetIsActive)
    ;[1 1 1] Tell the game state when the player enters and leaves this zone
    (Class|BPIZoneStateMessage|PlayerEnteredZone(Message) (Game|GetGameState) self)))

(fn ConstructionScript)

(fn PrintInfo
  (params (Message :type String))
  ;[1 1 1] Prints a message with the zone name
  (Development|PrintString (Utilities|String|Append (Utilities|String|Append (Utilities|String|ToString(Name) (Variables|Default|GetZoneName)) ": ") Message)))

(fn GetSpawnerName
  (return (Variables|Default|GetZoneName)))