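; Base wall-buy actor that sells a weapon, or reserve ammo to players who already own it, for points.
; BeginPlay resolves the weapon and display name from ItemSold through map lookups, and the overlap volume shows or clears the matching price prompt.
; Interacting checks ownership, ammo status and points, then reports failure or charges through the GameMode and grants the purchase, using message calls to the player.
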(event OnComponentBeginOverlap(InteractionVolume)
  (params (OverlappedComponent :type Primitive%20Component%20Object%20Reference) (OtherActor :type Actor%20Object%20Reference) (OtherComp :type Primitive%20Component%20Object%20Reference) (OtherBodyIndex :type Integer) (bFromSweep :type Boolean) (SweepResult :type Hit%20Result%20Structure%20%28by%20ref%29))
  (CallFunction|PromptPlayer OtherActor))

(event OnComponentEndOverlap(InteractionVolume)
  (params (OverlappedComponent :type Primitive%20Component%20Object%20Reference) (OtherActor :type Actor%20Object%20Reference) (OtherComp :type Primitive%20Component%20Object%20Reference) (OtherBodyIndex :type Integer))
  (Class|BPIPromptible|StopPrompt(Message) OtherActor))

(event EventBeginPlay
  (bind _itemsold (Variables|Default|GetItemSold))
  (Variables|Default|SetWeaponSold (.Value (Utilities|Map|Find (Variables|Default|GetItemStructMapping) _itemsold)))
  (Variables|Default|SetItemName (.Value (Utilities|Map|Find (Variables|Default|GetItemNameMap) _itemsold))))

(event EventInteract
  (params (Interactor :type Pawn%20Object%20Reference))
  (CallFunction|OnInteract Interactor))

(fn ConstructionScript)

(fn PromptPlayer
  (params (Target :type Object%20Object%20Reference))
  (bind _owneditems (Class|BPIPurchaser|GetPurchasedItems(Message) Target))
  (if (Utilities|Array|ContainsItem _owneditems (Variables|Default|GetItemName))
    (Class|BPIPromptible|Prompt(Message) Target (Utilities|String|Append "Purchase ammo: " (Utilities|String|ToString(Integer) (Variables|Default|GetAmmoCost))) self)
    (return)
    (else
      (Class|BPIPromptible|Prompt(Message) Target (Utilities|String|Append "Purchase " (Utilities|String|ToString(Name) (Variables|Default|GetItemName)) ": " (Utilities|String|ToString(Integer) (Variables|Default|GetPurchaseCost))) self)
      (return))))

(fn OnInteract
  (params (Interactor :type Pawn%20Object%20Reference))
  (Utilities|FlowControl|Sequence
    (:then_0
      (LocalVariables|SetTheInteractor Interactor))
    (:then_1
      (bind _points (Class|BPIPurchaser|GetPoints(Message) (LocalVariables|GetTheInteractor)))
      (LocalVariables|SetPlayerPoints _points)
      (bind _owneditems (Class|BPIPurchaser|GetPurchasedItems(Message) (LocalVariables|GetTheInteractor)))
      (LocalVariables|SetPlayerItems _owneditems))
    (:then_2
      (if (Utilities|Array|ContainsItem (LocalVariables|GetPlayerItems) (Variables|Default|GetItemName))
        (bind _isreserveammofull (Class|BPIWeaponOwner|GetReserveAmmoStatus(Message) (LocalVariables|GetTheInteractor)))
        (if _isreserveammofull
          (Class|BPIPurchaser|PurchaseFailed(Message) (LocalVariables|GetTheInteractor) (Variables|Default|GetItemName) "NewEnumerator2")
          (return)
          (elif (>= (LocalVariables|GetPlayerPoints) (Variables|Default|GetAmmoCost))
            (Class|BPIStateMessageHandler|PlayerSpentPoints(Message) (Game|GetGameMode) (Pawn|GetController (LocalVariables|GetTheInteractor)) (Variables|Default|GetAmmoCost))
            (Class|BPIWeaponOwner|AwardReserveAmmo(Message) (LocalVariables|GetTheInteractor))
            (return)
            (else
              (Class|BPIPurchaser|PurchaseFailed(Message) (LocalVariables|GetTheInteractor) (Variables|Default|GetItemName) "NewEnumerator0")
              (return))))))
    (:then_3
      (if (>= (LocalVariables|GetPlayerPoints) (Variables|Default|GetPurchaseCost))
        (Class|BPIStateMessageHandler|PlayerSpentPoints(Message) (Game|GetGameMode) (Pawn|GetController (LocalVariables|GetTheInteractor)) (Variables|Default|GetPurchaseCost))
        (Class|BPIWeaponOwner|GiveWeapon(Message) (LocalVariables|GetTheInteractor) (Variables|Default|GetWeaponSold))
        (return)
        (else
          (Class|BPIPurchaser|PurchaseFailed(Message) (LocalVariables|GetTheInteractor) (Variables|Default|GetItemName) "NewEnumerator0")
          (return))))))