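; BP_GrenadeBuy is an interactable wall buy that sells grenade ammo to players for points.
; On Interact it queries the interactor's grenade status and points through message calls, avoiding a cast to the player class.
; A successful purchase reports the spend to the GameMode and awards ammo.
; A true grenade status or insufficient points instead sends the interactor a purchase-failed message with the item name and reason.
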(event EventBeginPlay)

(event Collision|EventActorBeginOverlap
  (params (OtherActor :type Actor%20Object%20Reference)))

(event EventTick
  (params (DeltaSeconds :type Float%20%28single-precision%29)))

(event EventInteract
  (params (Interactor :type Pawn%20Object%20Reference))
  (bind _isgrenadesfull (Class|BPIWeaponOwner|GetGrenadeStatus(Message) Interactor))
  (if _isgrenadesfull
    (Class|BPIPurchaser|PurchaseFailed(Message) Interactor (Variables|Default|GetItemName) "NewEnumerator2")
    (else
      (bind _points (Class|BPIPurchaser|GetPoints(Message) Interactor))
      (if (>= _points (Variables|Default|GetPurchaseCost))
        (Class|BPIStateMessageHandler|PlayerSpentPoints(Message) (Game|GetGameMode) (Pawn|GetController Interactor) (Variables|Default|GetPurchaseCost))
        (Class|BPIWeaponOwner|AwardGrenadeAmmo(Message) Interactor)
        (else
          (Class|BPIPurchaser|PurchaseFailed(Message) Interactor (Variables|Default|GetItemName) "NewEnumerator0"))))))

(fn ConstructionScript
  (|CallParentFunction))