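; BP_Grenade is an explosive projectile, filed under soda bottle weapons, that detonates on first contact.
; A hit or overlap on its Sphere, or a ProjectileMovement bounce (which also prints a debug string), feeds one shared explosion sequence.
; That sequence applies radial explosive damage credited to player controller 0, spawns the explosion emitter and sound, then destroys the actor.
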(event OnComponentHit(Sphere)
  (params (HitComponent :type Primitive%20Component%20Object%20Reference) (OtherActor :type Actor%20Object%20Reference) (OtherComp :type Primitive%20Component%20Object%20Reference) (NormalImpulse :type Vector :default "0, 0, 0") (Hit :type Hit%20Result%20Structure%20%28by%20ref%29))
  (bind _sphere (Variables|Default|GetSphere))
  (bind _returnvalue (Transformation|GetWorldLocation _sphere))
  (Game|Damage|ApplyRadialDamage (Variables|Default|GetFlatDamage) _returnvalue (Variables|Default|GetExplosiveRadius) "/Game/KZC/Weapons/DamageTypes/BP_DamageExplosive.BP_DamageExplosive_C" 0 self (Game|GetPlayerController 0) false "ECC_Visibility")
  (Effects|SpawnEmitteratLocation "/Game/StarterContent/Particles/P_Explosion.P_Explosion" _returnvalue)
  (Audio|PlaySoundatLocation "/Game/StarterContent/Audio/Explosion01.Explosion01" _returnvalue "0, 0, 0" 1.0 1.0 0.0 0 0 0 0)
  (Actor|DestroyActor))

(event OnComponentBeginOverlap(Sphere)
  (params (OverlappedComponent :type Primitive%20Component%20Object%20Reference) (OtherActor :type Actor%20Object%20Reference) (OtherComp :type Primitive%20Component%20Object%20Reference) (OtherBodyIndex :type Integer) (bFromSweep :type Boolean) (SweepResult :type Hit%20Result%20Structure%20%28by%20ref%29))
  (bind _sphere (Variables|Default|GetSphere))
  (bind _returnvalue (Transformation|GetWorldLocation _sphere))
  (Game|Damage|ApplyRadialDamage (Variables|Default|GetFlatDamage) _returnvalue (Variables|Default|GetExplosiveRadius) "/Game/KZC/Weapons/DamageTypes/BP_DamageExplosive.BP_DamageExplosive_C" 0 self (Game|GetPlayerController 0) false "ECC_Visibility")
  (Effects|SpawnEmitteratLocation "/Game/StarterContent/Particles/P_Explosion.P_Explosion" _returnvalue)
  (Audio|PlaySoundatLocation "/Game/StarterContent/Audio/Explosion01.Explosion01" _returnvalue "0, 0, 0" 1.0 1.0 0.0 0 0 0 0)
  (Actor|DestroyActor))

(event OnProjectileBounce(ProjectileMovement)
  (params (ImpactResult :type Hit%20Result%20Structure%20%28by%20ref%29) (ImpactVelocity :type Vector%20%28by%20ref%29 :default "0, 0, 0"))
  (bind _sphere (Variables|Default|GetSphere))
  (bind _returnvalue (Transformation|GetWorldLocation _sphere))
  (Development|PrintString "BOUNCE 
")
  (Game|Damage|ApplyRadialDamage (Variables|Default|GetFlatDamage) _returnvalue (Variables|Default|GetExplosiveRadius) "/Game/KZC/Weapons/DamageTypes/BP_DamageExplosive.BP_DamageExplosive_C" 0 self (Game|GetPlayerController 0) false "ECC_Visibility")
  (Effects|SpawnEmitteratLocation "/Game/StarterContent/Particles/P_Explosion.P_Explosion" _returnvalue)
  (Audio|PlaySoundatLocation "/Game/StarterContent/Audio/Explosion01.Explosion01" _returnvalue "0, 0, 0" 1.0 1.0 0.0 0 0 0 0)
  (Actor|DestroyActor))

(event EventBeginPlay)

(event Collision|EventActorBeginOverlap
  (params (OtherActor :type Actor%20Object%20Reference)))

(event EventTick
  (params (DeltaSeconds :type Float%20%28single-precision%29)))

(fn ConstructionScript)