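; Employee player controller for a zombie game that manages the player's points.
; On BeginPlay it casts its PlayerState to BP_ZombiePlayerState and caches it, printing a warning if the cast fails.
; GivePoints adds the gained amount to the cached state's Points, then PointsUpdated broadcasts the new total through the CallPointsUpdate dispatcher.
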(event Custom|PointsUpdated
  (Default|CallPointsUpdate (Variables|/Game/KZC/Blueprints/Framework/BP_ZombiePlayerState.BP_ZombiePlayerState_C|GetPoints (Variables|Default|GetZombiePlayerState))))

(event EventBeginPlay
  (bind _asbp_zombie_player_state (Utilities|Casting|CastToBP_ZombiePlayerState (Variables|GetPlayerState))
    (:then
      (Variables|Default|SetZombiePlayerState _asbp_zombie_player_state))
    (:CastFailed
      (Development|PrintString "EmployeeControllerDoesNotHaveZombiePlayerState" true true "(R=1.000000,G=0.048555,B=0.024679,A=1.000000)"))))

(event EventTick
  (params (DeltaSeconds :type Float%20%28single-precision%29)))

(event EventGivePoints
  (params (PointsGained :type Integer))
  (Variables|/Game/KZC/Blueprints/Framework/BP_ZombiePlayerState.BP_ZombiePlayerState_C|SetPoints (Variables|Default|GetZombiePlayerState) (+ (Variables|/Game/KZC/Blueprints/Framework/BP_ZombiePlayerState.BP_ZombiePlayerState_C|GetPoints (Variables|Default|GetZombiePlayerState)) PointsGained))
  (CallFunction|PointsUpdated))

(fn ConstructionScript)